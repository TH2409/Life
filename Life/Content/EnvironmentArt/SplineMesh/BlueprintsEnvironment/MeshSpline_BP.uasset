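; Construction-script spline mesh Blueprint that builds an editable road or track along a spline.
; It syncs the TrackData array to the spline point count, padding with defaults but trimming only one surplus entry per run.
; Each segment becomes a RoadMesh spline mesh component, with per-point bank, width and height, optional loop closure and toggleable collision.
; The debug point-number text is disconnected, and the event graph is empty.
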(fn `BuildTrackElement`
  (params (LoopIndex :type Integer) (TrackElementMesh :type "StaticMesh Object Reference"))
  (locals (LocalCurrentLoopIndex :type Integer) (LocalTrackElementMesh :type "StaticMesh Object Reference") (LocalNextLoopIndex :type Integer) (Local_StartLocation :type "Vector Structure" :default (0.0 0.0 0.0)) (Local_StartTangent :type "Vector Structure" :default (0.0 0.0 0.0)) (Local_EndLocation :type "Vector Structure" :default (0.0 0.0 0.0)) (Local_EndTangent :type "Vector Structure" :default (0.0 0.0 0.0)) (LocalCurrentSplineMesh :type "SplineMeshComponent Object Reference") (Local_StartRoll :type "Float (double-precision)") (Local_StartScale :type "Vector2D Structure") (Local_EndRoll :type "Float (double-precision)") (Local_EndScale :type "Vector2D Structure"))
  (bind (_location _tangent) (`SplineComponent.GetLocationAndTangentAtSplinePoint` (`self.Spline`) (`local.LocalNextLoopIndex`) "Local"))
  (bind (_location_2 _tangent_2) (`SplineComponent.GetLocationAndTangentAtSplinePoint` (`self.Spline`) (`local.LocalCurrentLoopIndex`) "Local"))
  (bind (_output_trackbank _output_tackwidth _output_trackheight) (break `/Game/EnvironmentArt/SplineMesh/BlueprintsEnvironment/TrackData` (`|GetArrayItem` (`self.TrackData`) (`local.LocalCurrentLoopIndex`))))
  (bind (_output_trackbank_2 _output_tackwidth_2 _output_trackheight_2) (break `/Game/EnvironmentArt/SplineMesh/BlueprintsEnvironment/TrackData` (`|GetArrayItem` (`self.TrackData`) (`local.LocalNextLoopIndex`))))
  (set `local.LocalCurrentLoopIndex` LoopIndex)
  (set `local.LocalNextLoopIndex` (mod (+ LoopIndex 1) (`self.NumberOfSplinePoints`)))
  (set `local.LocalTrackElementMesh` TrackElementMesh)
  (`|ExecutionSequence`
    (:`then_0`
      (set `local.Local_StartLocation` _location_2)
      (set `local.Local_StartTangent` _tangent_2)
      (set `local.Local_EndLocation` _location)
      (set `local.Local_EndTangent` _tangent)
      (set `local.Local_StartRoll` _output_trackbank)
      (set `local.Local_StartScale` (`KismetMathLibrary.MakeVector2D` _output_tackwidth _output_trackheight))
      (set `local.Local_EndRoll` _output_trackbank_2)
      (set `local.Local_EndScale` (`KismetMathLibrary.MakeVector2D` _output_tackwidth_2 _output_trackheight_2)))
    (:`then_1`
      (bind _returnvalue (`AddComponent|NODE_AddSplineMeshComponent-0`))
      (bind _output_get (set `local.LocalCurrentSplineMesh` _returnvalue))
      (`StaticMeshComponent.SetStaticMesh` _output_get (`local.LocalTrackElementMesh`))
      (`SplineMeshComponent.SetStartAndEnd` (`local.LocalCurrentSplineMesh`) (`local.Local_StartLocation`) (`local.Local_StartTangent`) (`local.Local_EndLocation`) (`local.Local_EndTangent`) true)
      (`SplineMeshComponent.SetStartRoll` (`local.LocalCurrentSplineMesh`) (`local.Local_StartRoll`) true)
      (`SplineMeshComponent.SetEndRoll` (`local.LocalCurrentSplineMesh`) (`local.Local_EndRoll`) true)
      (`SplineMeshComponent.SetStartScale` (`local.LocalCurrentSplineMesh`) (`local.Local_StartScale`) true)
      (`SplineMeshComponent.SetEndScale` (`local.LocalCurrentSplineMesh`) (`local.Local_EndScale`) true)
      (`PrimitiveComponent.SetCollisionEnabled` (`local.LocalCurrentSplineMesh`) (select `bool` (`self.Collisions`) :`false` "NoCollision" :`true` "QueryAndPhysics" :!type "ECollisionEnabled Enum")))))

(fn `UserConstructionScript`
  (bind _trackdata (`self.TrackData`))
  (`|ExecutionSequence`
    (:`then_0`
      (set `self.NumberOfSplinePoints` (`SplineComponent.GetNumberOfSplinePoints` (`self.Spline`))))
    (:`then_1`
      (`/Engine/EditorBlueprintResources/StandardMacros.CompareInt` (`KismetArrayLibrary.Array_Length` (`self.TrackData`)) (`self.NumberOfSplinePoints`) :!label _label
        (:`>`
          (`KismetArrayLibrary.Array_Remove` _trackdata (`KismetArrayLibrary.Array_LastIndex` _trackdata)))
        (:`<`
          (`KismetArrayLibrary.Array_Add` (`self.TrackData`) (`self.TrackDataDefaults`))
          (goto _label))))
    (:`then_2`
      (for _index (range (+ (- (`self.NumberOfSplinePoints`) (select `bool` (`self.LoopingTrack`) :`false` 2 :`true` 1)) 1))
        (`self.BuildTrackElement` _index (`self.RoadMesh`))))
    (:`then_3`
      (if (`self.Draw Track Point Numbers`)
        (for _index_2 (range (`self.NumberOfSplinePoints`))
          _)))))