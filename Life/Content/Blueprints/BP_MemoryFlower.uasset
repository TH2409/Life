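; Memory flower actor that grows on BeginPlay, then releases petal swarms linked to the father memory actors in the level.
; A Growth timeline drives growth and wind parameters on a dynamic material shared by the base and bud meshes.
; After timed delays, it spawns one BP_PetalSwarm per matching memory actor, passing it that actor and attaching it to the bud, and freezes the bud animation shortly afterward.
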(event `self.ReceiveBeginPlay`
  (`|ExecutionSequence`
    (:`then_0`
      (bind (_direction _stemgrowth _windspeed) (`Timeline|Growth`)
        (:`Update`
          (`MaterialInstanceDynamic.SetScalarParameterValue` (`self.FlowerMaterial`) "Growth" _stemgrowth)
          (`MaterialInstanceDynamic.SetScalarParameterValue` (`self.FlowerMaterial`) "WindIntensity" _windspeed)
          (`PrimitiveComponent.SetMaterial` (`self.SM_MemoryFlowerBase`) 0 (`self.FlowerMaterial`))
          (`PrimitiveComponent.SetMaterial` (`self.SM_MemoryFlowerBud`) 0 (`self.FlowerMaterial`)))))
    (:`then_1`
      (`KismetSystemLibrary.Delay` 5.95)
      (`SkeletalMeshComponent.SetPlayRate` (`self.SM_MemoryFlowerBud`) 0.0))
    (:`then_2`
      (`KismetSystemLibrary.Delay` 5.5)
      (bind _asbp_father_memory (castclass `/Game/Blueprints/BP_FatherMemory` "/Game/Blueprints/BP_FatherMemory.BP_FatherMemory_C"))
      (bind _outactors (`GameplayStatics.GetAllActorsOfClass` _asbp_father_memory))
      (for _index (range (+ (`KismetArrayLibrary.Array_LastIndex` _outactors) 1))
        (bind _returnvalue (`|SpawnActorFromClass` "/Game/Particles/BP_PetalSwarm.BP_PetalSwarm_C" (`self.GetTransform`) "Undefined" "OverrideRootScale"))
        (`/Game/Particles/BP_PetalSwarm.StoreBodyValues` _returnvalue (`|GetArrayItem` _outactors _index))
        (`/Game/Particles/BP_PetalSwarm.AttachtoBud` _returnvalue self)
        (`/Game/Particles/BP_PetalSwarm.SpawnParticle` _returnvalue)
        (set `self.MemoryInstances` (+ (`self.MemoryInstances`) 1))))))

(event `self.ReceiveTick`
  (params (DeltaSeconds :type "Float (single-precision)")))

(fn `UserConstructionScript`
  (bind _sm_memoryflowerbase (`self.SM_MemoryFlowerBase`))
  (bind _returnvalue (`PrimitiveComponent.CreateDynamicMaterialInstance` _sm_memoryflowerbase 0 "/Game/EnvironmentArt/Materials/M_MemFlower.M_MemFlower"))
  (bind _output_get (set `self.FlowerMaterial` _returnvalue))
  (`PrimitiveComponent.SetMaterial` _sm_memoryflowerbase 0 _output_get)
  (`PrimitiveComponent.SetMaterial` (`self.SM_MemoryFlowerBud`) 0 _output_get))