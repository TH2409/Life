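; BP_FatherMemory is a father memory actor whose skeletal mesh plays a timed bark and leaf growth effect when play begins.
; The construction script creates dynamic material instances for the bark and leaf slots from two family memory materials.
; BeginPlay zeroes each Growth parameter, then after a short delay a timeline animates bark growth, and a second, later-starting timeline animates leaf growth.
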(event `self.ReceiveBeginPlay`
  (`|ExecutionSequence`
    (:`then_0`
      (`MaterialInstanceDynamic.SetScalarParameterValue` (`self.Bark`) "Growth" 0.0)
      (`PrimitiveComponent.SetMaterial` (`self.SKM_FatherMemory`) 1 (`self.Bark`)))
    (:`then_1`
      (`MaterialInstanceDynamic.SetScalarParameterValue` (`self.Leaf`) "Growth" 0.0)
      (`PrimitiveComponent.SetMaterial` (`self.SKM_FatherMemory`) 0 (`self.Leaf`)))
    (:`then_2`
      (`KismetSystemLibrary.Delay` 3.0)
      (`|ExecutionSequence`
        (:`then_0`
          (bind (_direction _stemgrowth) (`Timeline|Timeline_0`)
            (:`Update`
              (`MaterialInstanceDynamic.SetScalarParameterValue` (`self.Bark`) "Growth" _stemgrowth)
              (`PrimitiveComponent.SetMaterial` (`self.SKM_FatherMemory`) 1 (`self.Bark`)))))
        (:`then_1`
          (`KismetSystemLibrary.Delay` 4.0)
          (bind (_direction_2 _stemgrowth_2) (`Timeline|Timeline_1`)
            (:`Update`
              (`MaterialInstanceDynamic.SetScalarParameterValue` (`self.Leaf`) "Growth" _stemgrowth_2)
              (`PrimitiveComponent.SetMaterial` (`self.SKM_FatherMemory`) 0 (`self.Leaf`)))))))))

(fn `UserConstructionScript`
  (bind _skm_fathermemory (`self.SKM_FatherMemory`))
  (`|ExecutionSequence`
    (:`then_0`
      (bind _returnvalue (`PrimitiveComponent.CreateDynamicMaterialInstance` _skm_fathermemory 1 "/Game/Characters/Materials/M_FamilyMemory.M_FamilyMemory"))
      (bind _output_get (set `self.Bark` _returnvalue))
      (`PrimitiveComponent.SetMaterial` (`self.SKM_FatherMemory`) 1 _output_get))
    (:`then_1`
      (bind _returnvalue_2 (`PrimitiveComponent.CreateDynamicMaterialInstance` _skm_fathermemory 0 "/Game/Characters/Materials/M_FamilyMemory1.M_FamilyMemory1"))
      (bind _output_get_2 (set `self.Leaf` _returnvalue_2))
      (`PrimitiveComponent.SetMaterial` (`self.SKM_FatherMemory`) 0 _output_get_2))))