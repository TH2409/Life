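; Petal swarm particle actor that sweeps a stream of petals up the father memory figure of a memory flower.
; AttachtoBud attaches the particle component to the flower bud's PetalSource socket, and StoreBodyValues caches foot, hip and head socket locations from the father mesh.
; SpawnParticle activates the particles, then two chained timelines lerp the "Attract" vector parameter foot to hip and hip to head before deactivating.
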(event `AttachtoBud`
  (params (`Memory Flower` :type "/Game/Blueprints/BP_MemoryFlower Object Reference"))
  (`SceneComponent.K2_AttachToComponent` (`self.P_PetalSwarm`) (`/Game/Blueprints/BP_MemoryFlower.SM_MemoryFlowerBud` `Memory Flower`) "PetalSource" "KeepRelative" "KeepRelative" "KeepRelative" true))

(event `self.ReceiveBeginPlay`)

(event `SpawnParticle`
  (bind _p_petalswarm (`self.P_PetalSwarm`))
  (bind _hiplocation (`self.HipLocation`))
  (`ActorComponent.Activate` (`self.P_PetalSwarm`) false)
  (bind (_direction _petalposition) (`Timeline|Timeline_0`)
    (:`Update`
      (`ParticleSystemComponent.SetVectorParameter` _p_petalswarm "Attract" (`|EaseFunction` "Linear" _petalposition (`self.FootLocation`) _hiplocation)))
    (:`Finished`
      (bind (_direction_2 _petalposition_2) (`Timeline|Timeline_1`)
        (:`Update`
          (`ParticleSystemComponent.SetVectorParameter` _p_petalswarm "Attract" (`|EaseFunction` "Linear" _petalposition_2 _hiplocation (`self.HeadLocation`))))
        (:`Finished`
          (`ActorComponent.Deactivate` _p_petalswarm))))))

(fn `StoreBodyValues`
  (params (MemoryFlower_BP :type "/Game/Blueprints/BP_FatherMemory Object Reference"))
  (bind _skm_fathermemory (`/Game/Blueprints/BP_FatherMemory.SKM_FatherMemory` MemoryFlower_BP))
  (set `self.FootLocation` (`SceneComponent.GetSocketLocation` _skm_fathermemory "PetalStart"))
  (set `self.HipLocation` (`SceneComponent.GetSocketLocation` _skm_fathermemory "PetalMid"))
  (set `self.HeadLocation` (`SceneComponent.GetSocketLocation` _skm_fathermemory "PetalEnd"))
  (return))

(fn `UserConstructionScript`)